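; Interactable lever that triggers an action on its linked Door, passing its CombIndex, after a timed delay.
; Interact runs the parent logic and opens a gate, letting Tick fill the Progress widget over ActionDelay while counting down its remaining duration.
; On completion the widget resets, the Door action fires and the gate closes.
; Tick also hides the widget unless the player is within 500 units.
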(event `self.ReceiveTick`
  (params (DeltaSeconds :type "Float (single-precision)"))
  (bind _actiondelay (`self.actionDelay`))
  (bind _asprogress (cast `/Game/Blueprints/Widgets/Progress` (`WidgetComponent.GetUserWidgetObject` (`self.Widget`)) :!pure true))
  (bind _percent (`/Game/Blueprints/Widgets/Progress.percent` _asprogress))
  (bind _returnvalue (+ _percent (/ DeltaSeconds _actiondelay)))
  (`SceneComponent.SetHiddenInGame` (`self.Widget`) (>= (`KismetMathLibrary.Sqrt` (`self.GetSquaredDistanceTo` (`GameplayStatics.GetPlayerPawn` 0))) 500.0) false)
  (`/Engine/EditorBlueprintResources/StandardMacros.Gate` true :!label _label
    (:`Exit`
      (if (>= _returnvalue 1.0)
        (set `/Game/Blueprints/Widgets/Progress.percent` 0.0 _asprogress)
        (set `/Game/Blueprints/Widgets/Progress.duration` _actiondelay _asprogress)
        (`/Game/Blueprints/Door.Action` (`self.door`) (`self.combIndex`))
        (goto _label :!via `Close`)
        (else
          (set `/Game/Blueprints/Widgets/Progress.percent` _returnvalue _asprogress)
          (set `/Game/Blueprints/Widgets/Progress.duration` (- _actiondelay (* _actiondelay _percent)) _asprogress))))))

(event `self.Interact`
  (`parent.Interact`)
  (goto _label :!via `Open`))

(event `self.ReceiveBeginPlay`
  (set `/Game/Blueprints/Widgets/Progress.duration` (`self.actionDelay`) (cast `/Game/Blueprints/Widgets/Progress` (`WidgetComponent.GetUserWidgetObject` (`self.Widget`)) :!pure true)))

(fn `UserConstructionScript`
  (`parent.UserConstructionScript`))