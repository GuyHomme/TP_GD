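; AudioClue is an actor that repeatedly plays a spatial sound as a clue, paired with a mesh that visually reacts to playback.
; Construction applies the configured sound, material and attenuation falloff distance.
; After a short start delay, Play raises the material's Speed vector, starts the audio and re-arms itself by timer after sound duration plus cooldown.
; When audio finishes, Speed resets to zero through a dynamic material instance.
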(event `self.ReceiveBeginPlay`
  (`KismetSystemLibrary.Delay` 2.0)
  (`self.Play`))

(event `self.Audio.OnAudioFinished`
  (bind _staticmesh (`self.StaticMesh`))
  (bind _returnvalue (`PrimitiveComponent.CreateDynamicMaterialInstance` _staticmesh 0 (`PrimitiveComponent.GetMaterial` _staticmesh 0)))
  (`MaterialInstanceDynamic.SetVectorParameterValue` _returnvalue "Speed" (make `LinearColor` 0.0)))

(fn `Play`
  (bind _staticmesh (`self.StaticMesh`))
  (bind _audio (`self.Audio`))
  (bind _returnvalue (`PrimitiveComponent.CreateDynamicMaterialInstance` _staticmesh 0 (`PrimitiveComponent.GetMaterial` _staticmesh 0)))
  (`MaterialInstanceDynamic.SetVectorParameterValue` _returnvalue "Speed" (make `LinearColor` 15.0 5.0))
  (if (`KismetSystemLibrary.IsValid` (`AudioComponent.Sound` _audio))
    (`AudioComponent.Play` _audio 0.0)
    (`KismetSystemLibrary.K2_SetTimer` null "Play" (+ (`SoundBase.Duration` (`self.sound`)) (`self.cooldown`)))))

(fn `UserConstructionScript`
  (bind _audio (`self.Audio`))
  (`AudioComponent.SetSound` _audio (`self.sound`))
  (bind _outattenuationsettings (`AudioComponent.BP_GetAttenuationSettingsToApply` _audio))
  (bind _structout (setmembers `SoundAttenuationSettings` :`StructRef` _outattenuationsettings :`FalloffDistance` (`self.distance`)))
  (set `AudioComponent.AttenuationOverrides` _structout _audio)
  (`PrimitiveComponent.SetMaterial` (`self.StaticMesh`) 0 (`self.mat`)))