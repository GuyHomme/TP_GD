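; Base interactable actor that highlights its static mesh while the first-person character is inside its trigger box.
; Box begin and end overlap events call Highlight, which tracks the Highlighted state and swaps the mesh's first material between the default and a green vertex-color view-mode material.
; The construction script applies the default material, and Interact is an empty event left for overrides.
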(event `self.Box.OnComponentBeginOverlap`
  (params (OverlappedComponent :type "PrimitiveComponent Object Reference") (OtherActor :type "Actor Object Reference") (OtherComp :type "PrimitiveComponent Object Reference") (OtherBodyIndex :type Integer) (bFromSweep :type Boolean) (SweepResult :type "HitResult Structure (by ref)"))
  (cast `/Game/FirstPersonBP/Blueprints/FirstPersonCharacter` OtherActor)
  (if (not (`self.highlighted`))
    (`self.Highlight` true)))

(event `self.Box.OnComponentEndOverlap`
  (params (OverlappedComponent :type "PrimitiveComponent Object Reference") (OtherActor :type "Actor Object Reference") (OtherComp :type "PrimitiveComponent Object Reference") (OtherBodyIndex :type Integer))
  (cast `/Game/FirstPersonBP/Blueprints/FirstPersonCharacter` OtherActor)
  (if (`self.highlighted`)
    (`self.Highlight` false)))

(event `Interact`
  ;[1 1 1] Override
)

(fn `Highlight`
  (params (enable :type Boolean))
  (bind _staticmesh (`self.StaticMesh`))
  (bind _output_get (set `self.highlighted` enable))
  (if _output_get
    (`PrimitiveComponent.SetMaterial` _staticmesh 0 "/Engine/EngineDebugMaterials/VertexColorViewMode_GreenOnly.VertexColorViewMode_GreenOnly")
    (else
      (`PrimitiveComponent.SetMaterial` _staticmesh 0 (`self.defaultMat`)))))

(fn `UserConstructionScript`
  (`PrimitiveComponent.SetMaterial` (`self.StaticMesh`) 0 (`self.defaultMat`)))