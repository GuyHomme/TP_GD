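; Combination-lock door that opens when Action receives indices in the order stored in CombOrder, then plays its sequence animation.
; The first input starts a timed Listening window, and a wrong index resets progress.
; If time expires before opening, the door enters Cooling, ignoring input until a second timer returns it to Closed.
; Colorize shows each state through the mesh material's Color parameter.
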(event `Action`
  (params (index :type Integer))
  (switch `/Game/Declaration/State_Door` (`self.state`)
    (:`NewEnumerator0`
      (bind _returnvalue (`KismetSystemLibrary.K2_SetTimer` null "Cool" (`self.listening`)))
      (set `self.state` "NewEnumerator1")
      (`self.Colorize`))
    (:`NewEnumerator1`
      _))
  (if (== index (`|GetArrayItem` (`self.combOrder`) (`self.currentIndex`)))
    ;[1 1 1 1 30] Successful combination check
    (bind _result (`/Engine/EditorBlueprintResources/StandardMacros.IncrementInt` (`self.currentIndex`))
      (:`  `
        (if (== (`KismetArrayLibrary.Array_Length` (`self.combOrder`)) _result)
          ;[1 1 1 1 30] Open
          (set `self.state` "NewEnumerator3")
          (`MovieSceneSequencePlayer.Play` (`LevelSequenceActor.SequencePlayer` (`self.animation`)))
          (`self.Colorize`))))
    (else
      ;[1 1 1] Reset
      (set `self.currentIndex` 0))))

(event `Stop`
  (`KismetSystemLibrary.K2_ClearAndInvalidateTimerHandle` (stale `Action` _returnvalue))
  (`KismetSystemLibrary.K2_SetTimer` null "Reboot" (`self.cooling`))
  (`self.Colorize`))

(fn `Colorize`
  (bind _staticmesh (`self.StaticMesh`))
  (switch `/Game/Declaration/State_Door` (`self.state`)
    (:`NewEnumerator0`
      (`MeshComponent.SetVectorParameterValueOnMaterials` _staticmesh "Color" (`KismetMathLibrary.Conv_LinearColorToVector` (struct :`R` 1.0 :`G` 0.936502 :`A` 1.0))))
    (:`NewEnumerator1`
      (`MeshComponent.SetVectorParameterValueOnMaterials` _staticmesh "Color" (`KismetMathLibrary.Conv_LinearColorToVector` (struct :`G` 0.810008 :`B` 1.0 :`A` 1.0))))
    (:`NewEnumerator2`
      (`MeshComponent.SetVectorParameterValueOnMaterials` _staticmesh "Color" (`KismetMathLibrary.Conv_LinearColorToVector` (struct :`R` 1.0 :`G` 0.01538 :`A` 1.0))))
    (:`NewEnumerator3`
      (`MeshComponent.SetVectorParameterValueOnMaterials` _staticmesh "Color" (`KismetMathLibrary.Conv_LinearColorToVector` (struct :`R` 0.11232 :`G` 1.0 :`A` 1.0))))))

(fn `Cool`
  (if (`|EnumInequality` (`self.state`) "NewEnumerator3")
    (set `self.state` "NewEnumerator2")
    (`self.Stop`)
    (set `self.currentIndex` 0)))

(fn `Reboot`
  (if (`|EnumInequality` (`self.state`) "NewEnumerator3")
    (set `self.state` "NewEnumerator0")
    (`self.Colorize`)))

(fn `UserConstructionScript`
  (`MeshComponent.SetVectorParameterValueOnMaterials` (`self.StaticMesh`) "Color" (`KismetMathLibrary.Conv_LinearColorToVector` (struct :`R` 1.0 :`G` 0.304293 :`A` 1.0))))